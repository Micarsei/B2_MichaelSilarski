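; Piggybank actor that collects coins and triggers the game win once enough are deposited.
; Each Tick it polls the CoinDetection volume for overlapping BP_Coin2 actors, destroys them, increments CoinsDeposited and updates a TextRender counter.
; When the count reaches exactly five, it finds BP_FirstPersonCharacter with GetActorOfClass and calls GameWin on it.
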(event `self.ReceiveTick`
  (params (DeltaSeconds :type "Float (single-precision)"))
  (bind _coins_deposited (`self.Coins Deposited`))
  (for _array_element (`PrimitiveComponent.GetOverlappingActors` (`self.CoinDetection`) "/Game/MinigameContent/BP_Coin2.BP_Coin2_C")
    (`self.K2_DestroyActor` _array_element)
    (set `self.Coins Deposited` (+ _coins_deposited 1.0))
    (`TextRenderComponent.K2_SetText` (`self.TextRender`) (`KismetTextLibrary.Conv_DoubleToText` _coins_deposited "HalfToEven"))
    (if (== (`self.Coins Deposited`) 5.0)
      (bind _returnvalue (`GameplayStatics.GetActorOfClass` "/Game/FirstPerson/Blueprints/BP_FirstPersonCharacter.BP_FirstPersonCharacter_C"))
      (`/Game/FirstPerson/Blueprints/BP_FirstPersonCharacter.GameWin` _returnvalue))))

(fn `UserConstructionScript`)