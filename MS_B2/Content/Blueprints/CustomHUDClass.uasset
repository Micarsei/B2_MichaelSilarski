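; CustomHUDClass is a HUD Blueprint that manages two test widgets, apparently for minigame UI.
; BeginPlay creates and stores both widgets up front without displaying them.
; Separate custom events add each widget to the viewport on demand, and RemoveHud clears all widgets at once.
; TestMinigameShowText sets the first widget visible; Tick, overlap and construction logic are empty.
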(event `self.ReceiveBeginPlay`
  ; Creating all widgets on game start to be added to viewport as needed
  (bind _returnvalue (`|CreateWidget` "/Game/FirstPerson/Blueprints/BP_TestWidget1.BP_TestWidget1_C"))
  (set `self.TestWidget1` _returnvalue)
  (bind _returnvalue_2 (`|CreateWidget` "/Game/FirstPerson/Blueprints/BP_TestWidget2.BP_TestWidget2_C"))
  (set `self.TestWidget2` _returnvalue_2))

(event `AddHudTest1`
  ; Events for adding the widgets as needed
  (`UserWidget.AddToViewport` (`self.TestWidget1`) 0))

(event `AddHudTest2`
  ; Events for adding the widgets as needed
  (`UserWidget.AddToViewport` (`self.TestWidget2`) 0))

(event `RemoveHud`
  ; event for removing any active widgets
  (`WidgetLayoutLibrary.RemoveAllWidgets`))

(fn `TestMinigameShowText`
  (`Widget.SetVisibility` (`self.TestWidget1`) "Visible"))

(fn `UserConstructionScript`)