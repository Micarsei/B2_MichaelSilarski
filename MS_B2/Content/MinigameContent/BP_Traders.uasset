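; Trader actor for a minigame that exchanges salt bags for coins.
; Every Tick it polls BagDetection for overlapping SaltBagInteractible actors, destroys each and spawns a BP_Coin2 at CoinSpawn.
; SpawnedCoin is set to None instead of the new coin, so the following call to enable physics on its Cylinder has no valid target.
; BeginPlay caches a BP_Coin reference that the trade logic never uses.
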(event `self.ReceiveBeginPlay`
  (bind _returnvalue (`GameplayStatics.GetActorOfClass` "/Game/MinigameContent/BP_Coin.BP_Coin_C"))
  (set `self.CoinRef` _returnvalue))

(event `self.ReceiveTick`
  (params (DeltaSeconds :type "Float (single-precision)"))
  (for _array_element (`PrimitiveComponent.GetOverlappingActors` (`self.BagDetection`) "/Game/MinigameContent/SaltBagInteractible.SaltBagInteractible_C")
    (`self.K2_DestroyActor` _array_element)
    (`|SpawnActorFromClass` "/Game/MinigameContent/BP_Coin2.BP_Coin2_C" (`SceneComponent.K2_GetComponentToWorld` (`self.CoinSpawn`)) "Undefined" "MultiplyWithRoot" null null)
    (bind _output_get (set `self.SpawnedCoin` null))
    (`PrimitiveComponent.SetSimulatePhysics` (`/Game/MinigameContent/BP_Coin.Cylinder` _output_get) true)))

(fn `UserConstructionScript`)