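; BP_Mill is a minigame mill that converts small salt items into salt bags.
; Every Tick it polls the SmallSaltDetection component for overlapping SmallSaltInteractible actors, rather than using overlap events.
; Each one found is destroyed and replaced by a SaltBagInteractible spawned at BagSpawn, with physics simulation enabled on the bag.
; The SmallSaltRef cached on BeginPlay feeds only an unused overlap check.
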(event `self.ReceiveBeginPlay`
  (bind _returnvalue (`GameplayStatics.GetActorOfClass` "/Game/MinigameContent/SmallSaltInteractible.SmallSaltInteractible_C"))
  (set `self.SmallSaltRef` _returnvalue))

(event `self.ReceiveTick`
  (params (DeltaSeconds :type "Float (single-precision)"))
  (for _array_element (`PrimitiveComponent.GetOverlappingActors` (`self.SmallSaltDetection`) "/Game/MinigameContent/SmallSaltInteractible.SmallSaltInteractible_C")
    (`self.K2_DestroyActor` _array_element)
    (bind _returnvalue (`|SpawnActorFromClass` "/Game/MinigameContent/SaltBagInteractible.SaltBagInteractible_C" (`SceneComponent.K2_GetComponentToWorld` (`self.BagSpawn`)) "Undefined" "MultiplyWithRoot" null null))
    (`PrimitiveComponent.SetSimulatePhysics` (`/Game/MinigameContent/SaltBagInteractible.SaltBag` _returnvalue) true)))

(fn `UserConstructionScript`)